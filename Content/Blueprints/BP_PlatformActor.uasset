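; BP_PlatformActor is a scrolling platform segment built at BeginPlay from randomly chosen sprite tiles.
; Start blocks are fixed-length and drop their hazard and score trigger; others get random length, hazard position and coin height, with trigger and coin at the far end.
; Tick reloads the save game every frame for the X scroll speed.
; A living player's first trigger overlap passes the tile count to the game mode's score update.
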(event OnComponentBeginOverlap(ScoreTrigger)
  (params (OverlappedComponent :type Primitive%20Component%20Object%20Reference) (OtherActor :type Actor%20Object%20Reference) (OtherComp :type Primitive%20Component%20Object%20Reference) (OtherBodyIndex :type Integer) (bFromSweep :type Boolean) (SweepResult :type Hit%20Result%20Structure%20%28by%20ref%29))
  (bind _asbp_my_character (Utilities|Casting|CastToBP_MyCharacter OtherActor))
  (if (and (not (Variables|/Game/Blueprints/BP_MyCharacter.BP_MyCharacter_C|GetIsDead? _asbp_my_character)) (not (Variables|Default|GetStartBlock?)))
    (Utilities|FlowControl|DoOnce false
      (:Completed
        (bind _asgm_my_game_mode (Utilities|Casting|CastToGM_MyGameMode (Game|GetGameMode)))
        (Default|UpdateScore _asgm_my_game_mode (Variables|Default|GetHorTiles))))))

(event EventBeginPlay
  (Utilities|FlowControl|Sequence
    (:then_0
      (Variables|Default|SetHorTiles (select (Variables|Default|GetStartBlock?) 10 (Math|Random|RandomIntegerinRange 4 6)))
      (for _index (range 0 (- (Variables|Default|GetHorTiles) 1))
        (bind _returnvalue (AddComponent|AddPaperSpriteComponent false (Math|Transform|MakeTransform (Math|Vector|MakeVector (* _index 2e+02) 0.0 0.0) "0, 0, 0" "1,1,1")))
        (Rendering|Components|Sprite|SetSprite _returnvalue (select (Math|Random|RandomBool) "/Game/Art/Sprites/Platform/Brace_007_Sprite.Brace_007_Sprite" "/Game/Art/Sprites/Platform/Brace_001_Sprite.Brace_001_Sprite"))))
    (:then_1
      (if (Variables|Default|GetStartBlock?)
        (Components|DestroyComponent (Variables|Default|GetHazard))
        (else
          ;[1 1 1] 随机生成刺和金币位置
          (Transformation|SetRelativeLocation (Variables|Default|GetHazard) (Math|Vector|MakeVector (* (Math|Random|RandomIntegerinRange 0 (- (Variables|Default|GetHorTiles) 1)) 2e+02) 0.0 0.0) false false)
          (Transformation|SetRelativeLocation (Variables|Default|GetScoreTrigger) (Math|Vector|MakeVector (* (- (Variables|Default|GetHorTiles) 1) 2e+02) 0.0 0.0) false false)
          (Transformation|SetRelativeLocation (Variables|Default|Getcoin) (Math|Vector|MakeVector (* (- (Variables|Default|GetHorTiles) 1) 2e+02) 0.0 (Math|Random|RandomFloatinRange 1.5e+02 7e+02)) false false))))))

(event EventTick
  (params (DeltaSeconds :type Float%20%28single-precision%29))
  (bind _returnvalue (SaveGame|LoadGamefromSlot "SaveGames"))
  (bind _asbp_score_save_games (Utilities|Casting|CastToBP_ScoreSaveGames _returnvalue))
  ;[1 1 1] 修改速度
  (Transformation|AddActorWorldOffset (Math|Vector|MakeVector (* DeltaSeconds (Variables|/Game/Blueprints/BP_ScoreSaveGames.BP_ScoreSaveGames_C|Getspeed _asbp_score_save_games)) 0.0 0.0)))

(fn ConstructionScript)