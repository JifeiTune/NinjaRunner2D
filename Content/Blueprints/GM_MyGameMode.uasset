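; Game mode that tracks the current score, best score and a ranked list of past scores.
; On BeginPlay it loads or creates the BP_ScoreSaveGames save and shows the WB_InGame HUD, which refreshes as points are added.
; GameOver saves any new best, inserts a qualifying score into PastScores by shifting entries, sets a Chinese rank message and opens WB_GameOver.
; An unconnected alternative version of the ranking logic remains in the graph.
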(event Custom|CheckSaveScore
  (bind _returnvalue (SaveGame|DoesSaveGameExist "SaveGames"))
  (if _returnvalue
    (bind _returnvalue_2 (SaveGame|LoadGamefromSlot "SaveGames"))
    (bind _asbp_score_save_games (Utilities|Casting|CastToBP_ScoreSaveGames _returnvalue_2))
    (bind _output_get (Variables|Default|SetRef _asbp_score_save_games))
    (Variables|Default|SetBestScore (Variables|/Game/Blueprints/BP_ScoreSaveGames.BP_ScoreSaveGames_C|GetHighScore _output_get))
    (else
      (bind _returnvalue_3 (SaveGame|CreateSaveGameObject "/Game/Blueprints/BP_ScoreSaveGames.BP_ScoreSaveGames_C"))
      (bind _output_get_2 (Variables|Default|SetRef _returnvalue_3))
      (bind _output_get_3 (Variables|/Game/Blueprints/BP_ScoreSaveGames.BP_ScoreSaveGames_C|SetHighScore _output_get_2 0))
      (Variables|Default|SetBestScore _output_get_3)
      (SaveGame|SaveGametoSlot _output_get_2 "SaveGames")))
  (Variables|Default|SetScore 0))

(event Custom|UpdateHighScore
  (bind _ref (Variables|Default|GetRef))
  (if (> (Variables|Default|GetScore) (Variables|Default|GetBestScore))
    (bind _output_get (Variables|Default|SetBestScore (Variables|Default|GetScore)))
    (Variables|/Game/Blueprints/BP_ScoreSaveGames.BP_ScoreSaveGames_C|SetHighScore _ref _output_get)
    (SaveGame|SaveGametoSlot _ref "SaveGames")))

(event Custom|UpdateScore
  (params (Value :type Integer))
  (Variables|Default|SetScore (+ Value (Variables|Default|GetScore)))
  (Default|UpdateScores (Variables|Default|GetGameHUDRef) (Variables|Default|GetScore) (Variables|Default|GetBestScore)))

(event Custom|GameOver
  (CallFunction|UpdateHighScore)
  (Default|UpdateScores (Variables|Default|GetGameHUDRef) (Variables|Default|GetScore) (Variables|Default|GetBestScore))
  (Variables|/Script/Engine.PlayerController|SetbShowMouseCursor (Game|GetPlayerController 0) true)
  (CallFunction|IfinRank)
  (bind _returnvalue (UserInterface|CreateWidget "/Game/UMG/WB_GameOver.WB_GameOver_C"))
  (bind _output_get (Variables|Default|SetGameOverWidgetReference _returnvalue))
  (UserInterface|Viewport|AddtoViewport _output_get 0))

(event Custom|if%20in%20rank
  (bind _ref (Variables|Default|GetRef))
  (bind _ref_2 (Variables|Default|GetRef))
  (bind _pastscores (Variables|/Game/Blueprints/BP_ScoreSaveGames.BP_ScoreSaveGames_C|GetpastScores _ref))
  (Variables|Default|Setindex -1)
  (bind (_array_element _array_index) (Utilities|Array|ForEachLoopwithBreak (Variables|/Game/Blueprints/BP_ScoreSaveGames.BP_ScoreSaveGames_C|GetpastScores (Variables|Default|GetRef)) :!label _label)
    (:LoopBody
      (if (>= (Variables|Default|GetScore) _array_element)
        (Variables|Default|Setindex (+ _array_index 1))
        (goto _label Break)))
    (:Completed
      (if (> (Variables|Default|Getindex) 0)
        (Variables|Default|SetrankTip (Utilities|String|BuildString(Integer) "" "恭喜上榜！ 
第" (Variables|Default|Getindex) "名"))
        (for _index (range (Variables|Default|Getindex) 9)
          (Utilities|Array|SetArrayElem _pastscores (- (+ 9 (Variables|Default|Getindex)) _index) (Utilities|Array|Get(acopy) _pastscores (- (- (+ 9 (Variables|Default|Getindex)) _index) 1))))
        (Utilities|Array|SetArrayElem (Variables|/Game/Blueprints/BP_ScoreSaveGames.BP_ScoreSaveGames_C|GetpastScores _ref_2) (- (Variables|Default|Getindex) 1) (Variables|Default|GetScore))
        (SaveGame|SaveGametoSlot _ref_2 "SaveGames")
        (else
          (Variables|Default|SetrankTip "很遗憾您未上榜"))))))

(event EventBeginPlay
  (CallFunction|CheckSaveScore)
  (bind _returnvalue (UserInterface|CreateWidget "/Game/UMG/WB_InGame.WB_InGame_C"))
  (bind _output_get (Variables|Default|SetGameHUDRef _returnvalue))
  (UserInterface|Viewport|AddtoViewport _output_get 0)
  (Default|UpdateScores (Variables|Default|GetGameHUDRef) (Variables|Default|GetScore) (Variables|Default|GetBestScore)))

(fn ConstructionScript)